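; Timeline marker for a rhythm-map event, such as lighting, rings or speed, defined by Time, Type and Value.
; UpdateTransform puts the mesh in a lane by Type and offsets the actor along negative Y by Time times note separation.
; UpdateEvent, also run on construction, picks the material by Type, using Value for light color and effect, and shows Value as text on speed events.
; GetProperties packs the three fields into an Event struct.
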(event Custom|UpdateEvent
  (bind _eventmesh (Variables|Default|GetEventMesh))
  (bind _type (Variables|Default|GetType))
  (bind _textrender (Variables|Default|GetTextRender))
  (CallFunction|UpdateTransform)
  (if (< _type 5)
    (Rendering|Material|SetMaterial _eventmesh 0 (Utilities|Select :Index (Variables|Default|GetValue) :Option%200 "/Game/Materials/Events/MI_light_off.MI_light_off" :Option%201 "/Game/Materials/Events/MI_light_on_blue.MI_light_on_blue" :Option%202 "/Game/Materials/Events/MI_light_on_blue_flash.MI_light_on_blue_flash" :Option%203 "/Game/Materials/Events/MI_light_on_blue_fade.MI_light_on_blue_fade" :Option%204 "/Game/Materials/M_structure_mat.M_structure_mat" :Option%205 "/Game/Materials/Events/MI_light_on_red.MI_light_on_red" :Option%206 "/Game/Materials/Events/MI_light_on_red_flash.MI_light_on_red_flash" :Option%207 "/Game/Materials/Events/MI_light_on_red_fade.MI_light_on_red_fade"))
    (Rendering|SetVisibility _textrender false false :!label _label)
    (elif (< _type 10)
      (Rendering|Material|SetMaterial _eventmesh 0 "/Game/Materials/Events/M_event_rings.M_event_rings")
      (goto _label)
      (else
        (Rendering|Material|SetMaterial _eventmesh 0 "/Game/Materials/Events/M_event_speed.M_event_speed")
        (Rendering|SetVisibility _textrender true false)
        (Rendering|Components|TextRender|SetText _textrender (Utilities|Text|ToText(Integer) (Variables|Default|GetValue) false true 1 2))))))

(event Custom|UpdateTransform
  (Transformation|SetRelativeLocation (Variables|Default|GetEventMesh) (Math|Vector|MakeVector (+ (* (Utilities|Select :Index (Variables|Default|GetType) :Option%200 0 :Option%201 1 :Option%202 2 :Option%203 3 :Option%204 4 :Option%205 0 :Option%206 0 :Option%207 0 :Option%208 5 :Option%209 6 :Option%2010 0 :Option%2011 0 :Option%2012 7 :Option%2013 8) 5e+01) 25.0) 0.0 25.0) false false)
  (Transformation|SetActorRelativeLocation (Math|Vector|MakeVector 0.0 (* (* (CallFunction|GetNoteSep) (Variables|Default|GetTime)) -1.0) 0.0)))

(fn ConstructionScript
  (CallFunction|UpdateEvent))

(fn GetProperties
  (return (Utilities|Struct|MakeStructEvent (Variables|Default|GetTime) (Math|Conversions|ToFloat(Integer) (Variables|Default|GetType)) (Math|Conversions|ToFloat(Integer) (Variables|Default|GetValue)))))