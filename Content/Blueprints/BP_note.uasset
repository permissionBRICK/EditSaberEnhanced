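; Beat Saber-style note actor representing a red or blue cube, or a bomb, in a rhythm map.
; The construction script runs UpdateNote, which sets mesh, materials and arrow or dot from Type and Direction, then calls UpdateTransform.
; UpdateTransform rotates the mesh by cut direction, places it on a 4x3 Line/Layer grid wrapped by FixValues, and offsets the actor along -Y by Time.
; GetProperties returns the note's fields as a struct.
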(event Custom|Update%20Note
  (bind _arrow (Variables|Default|GetArrow))
  (bind _arrow_2 (Variables|Default|GetArrow))
  (bind _mesh (Variables|Default|GetMesh))
  (CallFunction|FixValues)
  (Utilities|FlowControl|Sequence
    (:then_0
      (switch int (Variables|Default|GetType)
        (:0
          (Components|StaticMesh|SetStaticMesh _mesh "/Game/Meshes/SM_CubeNote.SM_CubeNote")
          (Rendering|Material|SetMaterial _mesh 0 "/Game/Materials/M_CubeNote_red.M_CubeNote_red")
          (Rendering|Material|SetMaterial _arrow_2 0 "/Game/Materials/M_Arrow_red.M_Arrow_red")
          (if (== (Variables|Default|GetDirection) 8) :!label _label
            (Components|StaticMesh|SetStaticMesh _arrow "/Game/Meshes/SM_point.SM_point")
            (Transformation|SetRelativeLocation _arrow "0,25.000000,0.000000" false false)
            (else
              (Components|StaticMesh|SetStaticMesh _arrow "/Game/Meshes/SM_Arrow.SM_Arrow")
              (Transformation|SetRelativeLocation _arrow "0,25.000000,10.000000" false false))))
        (:1
          (Components|StaticMesh|SetStaticMesh _mesh "/Game/Meshes/SM_CubeNote.SM_CubeNote")
          (Rendering|Material|SetMaterial _mesh 0 "/Game/Materials/M_CubeNote_blue.M_CubeNote_blue")
          (Rendering|Material|SetMaterial _arrow_2 0 "/Game/Materials/M_Arrow_blue.M_Arrow_blue")
          (goto _label))
        (:3
          (Components|StaticMesh|SetStaticMesh _mesh "/Game/Meshes/SM_Bomb.SM_Bomb")
          (Rendering|Material|SetMaterial _mesh 0 "/Game/Materials/M_bomb.M_bomb")
          (Rendering|SetVisibility (Variables|Default|GetArrow) false false))))
    (:then_1
      (CallFunction|UpdateTransform))))

(event Custom|UpdateTransform
  (CallFunction|FixValues)
  (Utilities|FlowControl|Sequence
    (:then_0
      (Transformation|SetRelativeRotation (Variables|Default|GetMesh) (Math|Rotator|MakeRotator 0.0 (Utilities|Select :Index (Variables|Default|GetDirection) :Option%200 1.8e+02 :Option%201 0.0 :Option%202 2.7e+02 :Option%203 9e+01 :Option%204 225.0 :Option%205 135.0 :Option%206 315.0 :Option%207 45.0 :Option%208 0.0) 0.0) false false))
    (:then_1
      (Transformation|SetRelativeLocation (Variables|Default|GetMesh) (Math|Vector|MakeVector (- (* (Variables|Default|GetLine) 7e+01) 105.0) 0.0 (* (Variables|Default|GetLayer) 7e+01)) false false)
      (Transformation|SetActorRelativeLocation (Math|Vector|MakeVector 0.0 (* (* (CallFunction|GetNoteSep) (Variables|Default|GetTime)) -1.0) 0.0)))))

(fn ConstructionScript
  (CallFunction|UpdateNote))

(fn GetProperties
  (return (Utilities|Struct|MakeStructNote (Variables|Default|GetTime) (Variables|Default|GetLine) (Variables|Default|GetLayer) (Variables|Default|GetType) (Variables|Default|GetDirection))))

(fn FixValues
  (Variables|Default|SetLine (select (< (Math|Integer|%(Integer) (Variables|Default|GetLine) 4) 0) 3 (Math|Integer|%(Integer) (Variables|Default|GetLine) 4)))
  (Variables|Default|SetLayer (select (< (Math|Integer|%(Integer) (Variables|Default|GetLayer) 3) 0) 2 (Math|Integer|%(Integer) (Variables|Default|GetLayer) 3))))