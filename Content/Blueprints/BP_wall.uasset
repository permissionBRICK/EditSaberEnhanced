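; BP_wall is an obstacle wall actor for what appears to be a lane-based rhythm map, placed by time and line index.
; UpdateWall, also run by the construction script, scales the mesh from width, duration and note separation, with Type choosing between a tall, low-set shape and a shorter, raised one.
; Line sets the mesh's lateral offset and Time the actor's position along negative Y.
; GetProperties packs these values into an Obstacle struct.
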(event Custom|UpdateWall
  (bind _type (Variables|Default|GetType))
  (bind _meshroot (Variables|Default|GetMeshRoot))
  (Transformation|SetWorldScale3D _meshroot (Math|Vector|MakeVector (/ (* (Variables|Default|GetWidth) 7e+01) 1e+02) (* (Variables|Default|GetDuration) (/ (CallFunction|GetNoteSep) 1e+02)) (/ (Utilities|Select :Index _type :Option%200 2.8e+02 :Option%201 1.4e+02) 1e+02)))
  (Transformation|SetRelativeLocation _meshroot (Math|Vector|MakeVector (* (Variables|Default|GetLine) 7e+01) 0.0 (Utilities|Select :Index _type :Option%200 -4e+01 :Option%201 1e+02)) false false)
  (Transformation|SetActorRelativeLocation (Math|Vector|MakeVector -1.4e+02 (* (* (CallFunction|GetNoteSep) (Variables|Default|GetTime)) -1.0) 0.0)))

(fn ConstructionScript
  (CallFunction|UpdateWall))

(fn GetProperties
  (return (Utilities|Struct|MakeStructObstacle (Variables|Default|GetTime) (Variables|Default|GetLine) (Variables|Default|GetType) (Variables|Default|GetDuration) (Variables|Default|GetWidth))))